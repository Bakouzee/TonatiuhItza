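; Destructible vase used in a puzzle, where breaking the correct vase opens the GrilleOpenhearingRoom gate.
; On fracture of the destructible component, a WinningVase flag selects a winning or losing sound.
; A winning break also finds the gate actor by class and sets its Open flag.
; Both sounds are stopped on BeginPlay so they only play when the vase breaks.
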(event `self.ReceiveBeginPlay`
  (`AudioComponent.Stop` (`self.SoundWinning`))
  (`AudioComponent.Stop` (`self.SoundLosing`)))

(event `self.DestructibleComponent.OnComponentFracture`
  (params (HitPoint :type "Vector Structure (by ref)") (HitDirection :type "Vector Structure (by ref)"))
  (if (`self.WinningVase`)
    (`AudioComponent.Play` (`self.SoundWinning`) 0.0)
    (bind _returnvalue (`GameplayStatics.GetActorOfClass` "/Game/GrilleOpenhearingRoom.GrilleOpenhearingRoom_C"))
    (set `/Game/GrilleOpenhearingRoom.Open` true _returnvalue)
    (else
      (`AudioComponent.Play` (`self.SoundLosing`) 0.0))))

(fn `UserConstructionScript`)