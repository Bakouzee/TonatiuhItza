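; Trigger Blueprint for a hearing room that plays a sound associated with a compass direction.
; On BeginPlay, the Direction value selects the North, South, West or East sound and assigns it to the SoundDirection audio component.
; Any actor overlap plays that sound from the start, unless it is already playing.
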(event `self.ReceiveBeginPlay`
  (bind _sounddirection (`self.SoundDirection`))
  (switch `/Game/Prefabs/EnumDirections` (`self.Direction`)
    (:`NewEnumerator0`
      (`AudioComponent.SetSound` _sounddirection (`self.NorthSound`)))
    (:`NewEnumerator1`
      (`AudioComponent.SetSound` _sounddirection (`self.SouthSound`)))
    (:`NewEnumerator2`
      (`AudioComponent.SetSound` _sounddirection (`self.WestSound`)))
    (:`NewEnumerator3`
      (`AudioComponent.SetSound` _sounddirection (`self.EastSound`)))))

(event `self.ReceiveActorBeginOverlap`
  (params (OtherActor :type "Actor Object Reference"))
  (bind _sounddirection (`self.SoundDirection`))
  (if (not (`AudioComponent.IsPlaying` _sounddirection))
    (`AudioComponent.Play` _sounddirection 0.0)))

(fn `UserConstructionScript`)