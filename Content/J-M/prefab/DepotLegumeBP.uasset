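; DepotLegumeBP is a vegetable drop-off actor that judges a win or loss when a LegumesBP overlaps it.
; Each overlap walks ListATrouver, incrementing I for each of the first four entries and setting the onion, artichoke, apple and rotten-fruit flags.
; Only the onion flag compares against the item's Legume; the other three are set unconditionally.
; Tick prints "gagner" or "perdu" every frame while I equals 4.
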(event `self.ReceiveActorBeginOverlap`
  (params (OtherActor :type "Actor Object Reference"))
  (bind _aslegumes_bp (cast `/Game/J-M/prefab/LegumesBP` OtherActor))
  (for (_array_element _array_index) (`self.ListATrouver`)
    (switch `int` _array_index
      (:`0`
        (set `self.i` (+ (`self.i`) 1))
        (if (`|EnumEquality` _array_element (`/Game/J-M/prefab/LegumesBP.Legume` _aslegumes_bp))
          (set `self.isOignon` true)))
      (:`1`
        (set `self.i` (+ (`self.i`) 1))
        (if true
          (set `self.isArtichaut` true)))
      (:`2`
        (set `self.i` (+ (`self.i`) 1))
        (if true
          (set `self.isPomme` true)))
      (:`3`
        (set `self.i` (+ (`self.i`) 1))
        (if true
          (set `self.isFruitPourri` true))))))

(event `self.ReceiveTick`
  (params (DeltaSeconds :type "Float (single-precision)"))
  (if (== (`self.i`) 4)
    (if (and (`self.isOignon`) (`self.isArtichaut`) (`self.isPomme`) (`self.isFruitPourri`))
      (`KismetSystemLibrary.PrintString` "gagner")
      (else
        (`KismetSystemLibrary.PrintString` "perdu")))))

(fn `UserConstructionScript`)